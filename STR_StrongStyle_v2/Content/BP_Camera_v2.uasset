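; Shared basketball game camera that frames up to six players by following their midpoint and zooming with their spread.
; On BeginPlay it destroys default cameras, caches players from BP_GameState and becomes every player controller's view target.
; A fast looping timer sets spring arm length to the clamped largest pairwise player distance and interpolates the actor toward the average position.
; UpdateClassSetup re-runs the player and view-target setup.
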(event `self.ReceiveBeginPlay`
  ;[1 1 1] BEGIN PLAY
  (`/Engine/EditorBlueprintResources/StandardMacros.DoOnce` false
    (:`Completed`
      (`self.Initial Camera Setup`))))

(event `Initial Camera Setup`
  ;[1 1 1] INITIAL CAMERA SETUP: Clear other cameras,
  (`KismetSystemLibrary.PrintString` "CAMERA: Initial Camera Setup" true true (`self.DebugColor`) (`self.DebugDuration`))
  (`KismetSystemLibrary.Delay` 0.1)
  (`self.ClearCamerasDefault`)
  (`self.ClassSetup`)
  (`KismetSystemLibrary.K2_SetTimer` null "UpdateCamera" 0.01 true) ; Refreshing less than tick (.001)
)

(event `UpdateCamera`
  ;[1 1 1] UPDATE CAMERA: Adjust Arm Lengths based on Player Numbers
  (`self.SetArmLength`)
  (`self.SetCameraPos`)
  (`/Engine/EditorBlueprintResources/StandardMacros.DoOnce` false
    (:`Completed`
      (`KismetSystemLibrary.PrintString` "CAMERA: First update" true true (`self.DebugColor`) (`self.DebugDuration`)))))

(event `UpdateClassSetup`
  ;[1 1 1] UPDATE CLASS SETUP
  (`self.ClassSetup`))

(fn `CalculateDistance`
  (params (PlayerRef1 :type "/Game/BLUEPRINT/PLAYERS/BP_BasketballPlayer_M Object Reference") (PlayerRef2 :type "/Game/BLUEPRINT/PLAYERS/BP_BasketballPlayer_M Object Reference"))
  (returns (Distance1 :type "Float (double-precision)"))
  (locals (Distance :type "Float (double-precision)" :default 0.0))
  (if (and (`KismetSystemLibrary.IsValid` PlayerRef1) (`KismetSystemLibrary.IsValid` PlayerRef2))
    (set `local.Distance` (`self.GetDistanceTo` PlayerRef1 PlayerRef2))
    (else
      (set `local.Distance` 0.0)))
  (return (`local.Distance`)))

(fn `ClassSetup`
  (locals (DEBUGPlayerRefReadout :type String))
  (`KismetSystemLibrary.PrintString` (`KismetStringLibrary.Concat_StrStr` "CAMERA: " (`KismetSystemLibrary.GetObjectName` self) "running Class Setup") true true (`self.DebugColor`) (`self.DebugDuration`))
  ;[1 1 1] Get GS Player ref
  (bind _asbp_game_state (cast `/Game/Blueprints/BP_GameState` (`GameplayStatics.GetGameState`)))
  (bind _output_get (set `self.BP_GameState` _asbp_game_state))
  (set `self.PlayersReference` (`/Game/Blueprints/BP_GameState.Players` _output_get))
  (bind _outactors (`GameplayStatics.GetAllActorsOfClass` "/Game/BLUEPRINT/BP_Basketball_PlayerController.BP_Basketball_PlayerController_C"))
  (`PlayerController.SetViewTargetWithBlend` _outactors self 0.0 "VTBlend_Linear" 0.0 false)
  (for (_array_element _array_index) (`self.PlayersReference`)
    (switch `int` _array_index
      (:`0`
        (set `self.P1` _array_element))
      (:`1`
        (set `self.P2` _array_element))
      (:`2`
        (set `self.P3` _array_element))
      (:`3`
        (set `self.P4` _array_element))
      (:`4`
        (set `self.P5` _array_element))
      (:`5`
        (set `self.P6` _array_element)))))

(fn `ClearCamerasBPCam`
  ;[1 1 1] Destroy other Game Cameras (Sweep)
  (`KismetSystemLibrary.PrintString` (`KismetStringLibrary.Concat_StrStr` "Clearing game Cameras on" (`KismetSystemLibrary.GetObjectName` self)) true true (`self.DebugColor`) (`self.DebugDuration`))
  (bind _outactors (`GameplayStatics.GetAllActorsOfClass` (`self.DestroyCameraClassBP`)))
  (for _array_element _outactors
    (`self.K2_DestroyActor` _array_element)
    (`KismetSystemLibrary.PrintString` (`KismetStringLibrary.Concat_StrStr` "Camera " (`KismetSystemLibrary.GetDisplayName` _array_element) " destroyed") true true (`self.DebugColor`) (`self.DebugDuration`)))
  (`KismetSystemLibrary.PrintString` "CAMERA: Cameras Destroyed" true true (`self.DebugColor`) (`self.DebugDuration`)))

(fn `ClearCamerasDefault`
  ;[1 1 1] Destroy other Game Cameras (Sweep)
  (`KismetSystemLibrary.PrintString` (`KismetStringLibrary.Concat_StrStr` "Clearing game Cameras on" (`KismetSystemLibrary.GetObjectName` self)) true true (struct :`R` 1.0 :`B` 0.786197 :`A` 1.0) 10.0)
  (bind _outactors (`GameplayStatics.GetAllActorsOfClass` (`self.DestroyCameraClassDefault`)))
  (for _array_element _outactors
    (`self.K2_DestroyActor` _array_element)
    (`KismetSystemLibrary.PrintString` (`KismetStringLibrary.Concat_StrStr` "Camera " (`KismetSystemLibrary.GetDisplayName` _array_element) " destroyed") true true (`self.DebugColor`) (`self.DebugDuration`)))
  (`KismetSystemLibrary.PrintString` "CAMERA: Cameras Destroyed" true true (`self.DebugColor`) (`self.DebugDuration`)))

(fn `GetLocation`
  (params (Player :type "/Game/BLUEPRINT/PLAYERS/BP_BasketballPlayer_M Object Reference"))
  (returns (PlayerLocation :type "Vector Structure"))
  (locals (Location :type "Vector Structure" :default (0.0 0.0 0.0)))
  (`/Engine/EditorBlueprintResources/StandardMacros.IsValid` Player
    (:`Is Valid`
      (set `local.Location` (`self.K2_GetActorLocation` Player))
      (return (`local.Location`)))
    (:`Is Not Valid`
      (set `local.Location` (0.0 0.0 0.0)))))

(fn `SetArmLength`
  (bind _p1 (`self.P1`))
  (bind _p2 (`self.P2`))
  (bind _p3 (`self.P3`))
  (bind _p4 (`self.P4`))
  (bind _p5 (`self.P5`))
  (bind _p6 (`self.P6`))
  (set `SpringArmComponent.TargetArmLength` (`KismetMathLibrary.FClamp` (`.MaxValue` (`KismetMathLibrary.MaxOfFloatArray` (`|MakeArray` (`self.CalculateDistance` _p1 _p2) (`self.CalculateDistance` _p1 _p3) (`self.CalculateDistance` _p1 _p4) (`self.CalculateDistance` _p1 _p5) (`self.CalculateDistance` _p1 _p6) (`self.CalculateDistance` _p2 _p3) (`self.CalculateDistance` _p2 _p4) (`self.CalculateDistance` _p2 _p5) (`self.CalculateDistance` _p2 _p6) (`self.CalculateDistance` _p3 _p4) (`self.CalculateDistance` _p3 _p5) (`self.CalculateDistance` _p3 _p6) (`self.CalculateDistance` _p4 _p5) (`self.CalculateDistance` _p4 _p6) (`self.CalculateDistance` _p5 _p6)))) (`self.MinArmLength`) (`self.MaxArmLength`)) (`self.SpringArm`)))

(fn `SetCameraPos`
  (set `self.TargetPos` (/ (+ (`self.GetLocation` (`self.P1`)) (`self.GetLocation` (`self.P2`)) (`self.GetLocation` (`self.P3`)) (`self.GetLocation` (`self.P4`)) (`self.GetLocation` (`self.P5`)) (`self.GetLocation` (`self.P6`))) (`KismetMathLibrary.Conv_IntToDouble` (`KismetArrayLibrary.Array_Length` (`self.PlayersReference`)))))
  (`self.K2_SetActorLocation` (`KismetMathLibrary.VInterpTo` (`self.PreviousPos`) (`self.TargetPos`) (`GameplayStatics.GetWorldDeltaSeconds`) (`self.InterpSpeed`)))
  (set `self.PreviousPos` (`self.K2_GetActorLocation`)))

(fn `UserConstructionScript`)