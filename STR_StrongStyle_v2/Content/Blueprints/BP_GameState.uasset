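; Game state Blueprint for a basketball game that keeps the list of players and updates cameras when players join.
; A refresh event, run only with authority, rebuilds the Players array from all actors of the player class and prints the names for debugging.
; A separate event finds all camera actors and calls their class setup update when the GameMode signals a new player.
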(event `EventGS RefreshPlayers`
  ;[1 1 1] Refresh List of Players
  (`/Engine/EditorBlueprintResources/ActorMacros.Switch Has Authority`
    (:`Authority`
      (`self.RefreshPlayerArray`))))

(event `UpdateLocalCameras`
  ;[1 1 1] UPDATE LOCAL CAMERA: Called from GM when new player joins, casts to any Cameras and calls Update Class Setup
  (bind _outactors (`GameplayStatics.GetAllActorsOfClass` (`self.CameraClass`)))
  (for _array_element _outactors
    (bind _asbp_camera_v_2 (cast `` _array_element))
    (`self.UpdateClassSetup` _asbp_camera_v_2))
  (`KismetSystemLibrary.PrintString` "GAMESTATE: Local Cameras updated" true true (`self.DebugColor`) (`self.DebugDuration`)))

(fn `AppendPlayerReadoutString`
  (params (Object :type "Object Object Reference"))
  (set `self.DebugPlayerReadoutString` (`KismetStringLibrary.Concat_StrStr` (`self.DebugPlayerReadoutString`) ", " (`KismetSystemLibrary.GetDisplayName` Object))))

(fn `RefreshPlayerArray`
  ;[1 1 1] Clear Player Array
  (`KismetArrayLibrary.Array_Clear` (`self.Players`)) ; Clear Player Array
  ;[1 1 1] Get Players
  (bind _outactors (`GameplayStatics.GetAllActorsOfClass` (`self.PlayerClass`)))
  (for _array_element _outactors
    (bind _asbp_basketball_player_m (cast `/Game/BLUEPRINT/PLAYERS/BP_BasketballPlayer_M` _array_element)
      (:`then`
        (`self.AppendPlayerReadoutString` _asbp_basketball_player_m) ; Add to Debug Readout
        ;[1 1 1] Add to Array
        (`KismetArrayLibrary.Array_AddUnique` (`self.Players`) _asbp_basketball_player_m) ; Add  Each Player to the Array
      )
      (:`CastFailed`
        (`KismetSystemLibrary.PrintString` "Refresh Player Cast Failed!" true true (`self.DebugColorFailed`) (`self.DebugDuration`)))))
  ;[1 1 1] End and Print player list
  (`KismetSystemLibrary.PrintString` (`KismetStringLibrary.Concat_StrStr` "GAMESTATE: Refresh Player array results:" (`self.DebugPlayerReadoutString`)) true true (`self.DebugColor`) (`self.DebugDuration`)) ; Debug Player List
  (set `self.DebugPlayerReadoutString` ""))

(fn `UserConstructionScript`)