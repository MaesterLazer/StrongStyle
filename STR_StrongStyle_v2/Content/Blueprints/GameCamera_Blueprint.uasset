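; GameCamera_Blueprint is a camera actor that follows a target actor along the world Y axis while turning toward it.
; Each Tick it sets the root component's yaw from a look-at rotation to LookAtTarget, keeping pitch and roll unchanged.
; It then matches the target's Y position while holding its own X and Z, with no smoothing.
; SetLookAtTarget assigns the actor to track.
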(event `self.ReceiveTick`
  (params (DeltaSeconds :type "Float (single-precision)"))
  (bind _returnvalue (`self.K2_GetActorLocation`))
  (bind _rootcomponent (`self.RootComponent`))
  (bind _returnvalue_2 (`self.K2_GetActorLocation` (`self.LookAtTarget`)))
  ;[1 1 1] Look At Target
  (`SceneComponent.K2_SetWorldRotation` _rootcomponent (`KismetMathLibrary.MakeRotator` (.roll (`SceneComponent.K2_GetComponentRotation` _rootcomponent)) (.pitch (`SceneComponent.K2_GetComponentRotation` _rootcomponent)) (.yaw (`KismetMathLibrary.FindLookAtRotation` _returnvalue _returnvalue_2))) false false)
  (`SceneComponent.K2_SetWorldLocation` _rootcomponent (`KismetMathLibrary.MakeVector` (.x _returnvalue) (.y _returnvalue_2) (.z _returnvalue)) false false))

(fn `SetLookAtTarget`
  (params (`New Look At Target` :type "Actor Object Reference"))
  (set `self.LookAtTarget` `New Look At Target`))

(fn `UserConstructionScript`)