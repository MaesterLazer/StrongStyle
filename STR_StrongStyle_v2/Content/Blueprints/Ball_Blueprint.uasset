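; Ball actor that scores a basket when it passes out of a goal detector.
; On end overlap with an actor tagged GoalDetector, it casts to GoalDetector_Blueprint, reads that goal's team and updates the score UI.
; The begin-overlap Player check leads to no action, as the pickup logic here is disconnected and noted as handled in the Player Blueprint.
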(event `self.ReceiveActorBeginOverlap`
  (params (OtherActor :type "Actor Object Reference"))
  ;[1 1 1] Overlap Check
  ;;[1 1 1] Determine Overlapper
  (if (`self.ActorHasTag` OtherActor "Player")
    _))

(event `self.ReceiveActorEndOverlap`
  (params (OtherActor :type "Actor Object Reference"))
  ;[1 1 1] Overlap Check
  ;;[1 1 1] Determine Overlapper
  (if (`self.ActorHasTag` OtherActor "GoalDetector")
    (bind _asgoal_detector_blueprint (cast `/Game/Blueprints/GoalDetector_Blueprint` OtherActor))
    ;;[1 1 1] Score Basket
    (bind _teamnumber (`/Game/Blueprints/GoalDetector_Blueprint.Get Team` _asgoal_detector_blueprint))
    (`/Game/InGame_UIWidget.UpdateScore` (`self.ScoreUI`) _teamnumber)))

(fn `UserConstructionScript`)