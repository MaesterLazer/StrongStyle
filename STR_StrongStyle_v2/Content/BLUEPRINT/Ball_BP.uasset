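; Basketball actor that handles grabbing, launching, homing and scoring.
; Launches set physics velocity, boosting slow passes to a minimum horizontal speed, then detach the ball and re-enable grabbing and physics.
; Homing redirects velocity toward its target each Tick at constant speed until a hit or grab.
; On authority, grabs update game mode team phases, as do launches, and leaving a GoalDetector can update the scoreboard UI.
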(event `self.ReceiveBeginPlay`
  ;[1 1 1] Add UI and set Reference
  (bind _asbp_game_instance (cast `/Game/BLUEPRINT/BP_GameInstance` (`GameplayStatics.GetGameInstance`))
    (:`then`
      (`/Game/BLUEPRINT/BP_GameInstance.AddWidgetUI` _asbp_game_instance)
      (set `self.ScoreboardUI` (`/Game/BLUEPRINT/BP_GameInstance.ScoreboardUI` _asbp_game_instance)))
    (:`CastFailed`
      (`KismetSystemLibrary.PrintString` "Ball Game Instance Cast Failed!"))))

(event `self.ReceiveActorBeginOverlap`
  (params (OtherActor :type "Actor Object Reference"))
  ;[1 1 1] Overlap Check
  ;;[1 1 1] Determine Overlapper
  (if (`self.ActorHasTag` OtherActor "Player")
    _))

(event `self.ReceiveActorEndOverlap`
  (params (OtherActor :type "Actor Object Reference"))
  ;[1 1 1] Overlap Check
  ;;[1 1 1] Determine Overlapper
  (if (`self.ActorHasTag` OtherActor "GoalDetector")
    (`self.Score` OtherActor)))

(event `Score`
  (params (GoalDetector :type "Object Object Reference"))
  ;[1 1 1] Score Basket
  (`/Engine/EditorBlueprintResources/ActorMacros.Switch Has Authority`
    (:`Authority`
      (bind _asgoal_detector_bp (cast `/Game/BLUEPRINT/GoalDetector_BP` GoalDetector))
      (bind _bcanscore (`/Game/BLUEPRINT/GoalDetector_BP.GetScore` _asgoal_detector_bp))
      (if _bcanscore
        (`/Game/BLUEPRINT/GoalDetector_BP.ResetScoreTimer` _asgoal_detector_bp)
        (bind _teamnumber (`/Game/BLUEPRINT/GoalDetector_BP.Get Team` _asgoal_detector_bp))
        (`self.UpdateScore` _teamnumber)))))

(event `Event BallGrabBall`
  (params (GrabberTeam :type Integer))
  ;[1 1 1] Grab ball (no long grabbable)
  (`/Engine/EditorBlueprintResources/ActorMacros.Switch Has Authority`
    (:`Authority`
      (`self.EventStatus BallGrabbed`)
      (`self.Event BallCallGMPhaseUpdate` GrabberTeam))))

(event `self.StaticMeshComponent.OnComponentHit`
  (params (HitComponent :type "PrimitiveComponent Object Reference") (OtherActor :type "Actor Object Reference") (OtherComp :type "PrimitiveComponent Object Reference") (NormalImpulse :type "Vector Structure") (Hit :type "HitResult Structure (by ref)"))
  ;[1 1 1] BOUNCE EFFECTS
  (if (`self.bIsHoming`)
    (`self.EventStatus StopHoming`)))

(event `self.ReceiveTick`
  (params (DeltaSeconds :type "Float (single-precision)"))
  ;[1 1 1] TICK
  (if (`self.bIsHoming`)
    (`self.Event Homing`)))

(event `EventStatus Homing`
  (params (HomingTarget :type "Actor Object Reference"))
  ;[1 1 1] STATUS AND COLLISION "STATES"
  (set `self.HomingTarget` HomingTarget)
  (set `self.bIsHoming` true))

(event `EventOnline BallLaunch`
  (params (`Shot Velocity` :type "Vector Structure") (Target :type "Actor Object Reference") (Homing :type Boolean) (HomingTarget :type "Actor Object Reference") (Pass :type Boolean))
  ;[1 1 1] BALL FORCES (Launch/Homing)
  ;;[1 1 1 1 28] Local Ball Launch
  (`self.EventLocal BallLaunch` `Shot Velocity` Target Homing HomingTarget Pass))

(event `EventStatus ReleaseBall`
  ;[1 1 1] STATUS AND COLLISION "STATES"
  (set `self.bIsGrabbable` true)
  (`KismetSystemLibrary.PrintString` (`KismetStringLibrary.Concat_StrStr` "BALL > NOW GRABBABLE:"))
  (`self.K2_DetachFromActor` "KeepWorld" "KeepWorld" "KeepWorld")
  (`KismetSystemLibrary.PrintString` "BALL > DETACHED FROM ACTOR")
  (`PrimitiveComponent.SetCollisionProfileName` (`self.StaticMeshComponent`) "CustomBall")
  (`PrimitiveComponent.SetSimulatePhysics` (`self.StaticMeshComponent`) true)
  (`KismetSystemLibrary.PrintString` "BALL > SIMULATING PHYSICS"))

(event `UpdateScore`
  (params (ScoreTeam :type Integer))
  (`/Game/BLUEPRINT/WIDGETS/BPW_InGameUI.UpdateScore` (`self.ScoreboardUI`) ScoreTeam))

(event `EventLocal BallLaunch`
  (params (`Shot Velocity` :type "Vector Structure") (Target :type "Actor Object Reference") (Homing :type Boolean) (HomingTarget :type "Actor Object Reference") (Pass :type Boolean))
  (bind _staticmeshcomponent (`self.StaticMeshComponent`))
  (bind _returnvalue (`KismetMathLibrary.MakeVector` (.x `Shot Velocity`) (.y `Shot Velocity`)))
  (bind _returnvalue_2 (/ (`KismetMathLibrary.VSize` _returnvalue) (`self.PassMinVel`)))
  ;[1 1 1] BALL FORCES (Launch/Homing)
  ;;[1 1 1 1 28] Local Ball Launch
  (if Pass
    (if (< _returnvalue_2 1.0)
      (`KismetSystemLibrary.PrintString` "BALL > BOOSTING PASS VELOCITY")
      (`PrimitiveComponent.SetPhysicsLinearVelocity` _staticmeshcomponent (`KismetMathLibrary.MakeVector` (.x (/ _returnvalue _returnvalue_2)) (.y (/ _returnvalue _returnvalue_2)) (.z `Shot Velocity`)) false "None")
      (else
        (`PrimitiveComponent.SetPhysicsLinearVelocity` _staticmeshcomponent `Shot Velocity` false "None" :!label _label)))
    (else
      (goto _label)))
  (`KismetSystemLibrary.PrintString` "BALL > VELOCITY SET (TODO! Change to force)")
  (`self.LOCAL ReleaseBall`)
  (`self.Event BallCallGMPhaseUpdate` 0 true)
  (if Homing
    (`self.EventStatus Homing` HomingTarget)
    (`KismetSystemLibrary.PrintString` "BALL > PREPARING FOR HOMING")))

(event `Event BallCallGMPhaseUpdate`
  (params (OffenseTeam :type Integer) (bBallReleaseNoTeam :type Boolean))
  ;[1 1 1] Call GM Phase Update
  (bind _asbasket_ball_game_mode_local (cast `/Game/BasketBallGameMode_Local` (`GameplayStatics.GetGameMode`))
    (:`then`
      (`/Game/BasketBallGameMode_Local.Event UpdateAllPhaseAssignments` _asbasket_ball_game_mode_local OffenseTeam bBallReleaseNoTeam))
    (:`CastFailed`
      (`KismetSystemLibrary.PrintString` "BALL x GM PHASE CAST FAILED"))))

(event `EventStatus BallGrabbed`
  ;[1 1 1] STATUS AND COLLISION "STATES"
  ;;[1 1 1 1 28] Status: Ball Grabbed
  (set `self.bIsGrabbable` false)
  (`KismetSystemLibrary.PrintString` (`KismetStringLibrary.Concat_StrStr` "BALL > GRABBED, NOT GRABBABLE"))
  (`self.EventStatus StopHoming`))

(event `LOCAL ReleaseBall`
  ;[1 1 1] BALL FORCES (Launch/Homing)
  ;;[1 1 1 1 28] Local Release Ball
  (`self.EventStatus ReleaseBall`))

(event `EventStatus StopHoming`
  ;[1 1 1] STATUS AND COLLISION "STATES"
  ;;[1 1 1 1 28] Stop Homing
  (set `self.bIsHoming` false)
  (`KismetSystemLibrary.PrintString` "BALL > STOPPING HOMING"))

(event `Event Homing`
  ;[1 1 1] BALL FORCES (Launch/Homing)
  ;;[1 1 1 1 28] Homing
  (`PrimitiveComponent.SetPhysicsLinearVelocity` (`self.StaticMeshComponent`) (* (`KismetMathLibrary.GetForwardVector` (`KismetMathLibrary.FindLookAtRotation` (`SceneComponent.K2_GetComponentLocation` (`self.StaticMeshComponent`)) (`self.K2_GetActorLocation` (`self.HomingTarget`)))) (`KismetMathLibrary.VSize` (`self.GetVelocity` self))) false "None"))

(event `ONLINE ReleaseBall`
  ;[1 1 1] ONLINE Release Ball
  (`/Engine/EditorBlueprintResources/ActorMacros.Switch Has Authority`
    (:`Authority`
      (`self.LOCAL ReleaseBall`))))

(fn `UserConstructionScript`)