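; Throwable basketball actor that tracks whether it can be grabbed and reports baskets to the scoreboard.
; Ending overlap with a goal detector scores for that detector's team on authority, through the scoreboard widget obtained from the game instance.
; Shooting detaches the ball, enables physics and collision, applies velocity and releases it.
; Grab, release and the basic shot are authority-gated; the rotation-offset shot variant is not.
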(event `self.ReceiveBeginPlay`
  ;[1 1 1] Add UI and set Reference
  (bind _asbp_game_instance (cast `/Game/BLUEPRINT/BP_GameInstance` (`GameplayStatics.GetGameInstance`))
    (:`then`
      (`/Game/BLUEPRINT/BP_GameInstance.AddWidgetUI` _asbp_game_instance)
      (set `self.ScoreboardUI` (`/Game/BLUEPRINT/BP_GameInstance.ScoreboardUI` _asbp_game_instance)))
    (:`CastFailed`
      (`KismetSystemLibrary.PrintString` "Ball Game Instance Cast Failed!"))))

(event `self.ReceiveActorBeginOverlap`
  (params (OtherActor :type "Actor Object Reference"))
  ;[1 1 1] Overlap Check
  ;;[1 1 1] Determine Overlapper
  (if (`self.ActorHasTag` OtherActor "Player")
    _))

(event `self.ReceiveActorEndOverlap`
  (params (OtherActor :type "Actor Object Reference"))
  ;[1 1 1] Overlap Check
  ;;[1 1 1] Determine Overlapper
  (if (`self.ActorHasTag` OtherActor "GoalDetector")
    (`self.Score` OtherActor)))

(event `Score`
  (params (GoalDetector :type "Object Object Reference"))
  ;[1 1 1] Score Basket
  (`/Engine/EditorBlueprintResources/ActorMacros.Switch Has Authority`
    (:`Authority`
      (bind _asgoal_detector_bp (cast `/Game/BLUEPRINT/GoalDetector_BP` GoalDetector))
      (bind _teamnumber (`/Game/BLUEPRINT/GoalDetector_BP.Get Team` _asgoal_detector_bp))
      (`self.UpdateScore` _teamnumber))))

(event `UpdateScore`
  (params (ScoreTeam :type Integer))
  (`/Game/BLUEPRINT/WIDGETS/BPW_InGameUI.UpdateScore` (`self.ScoreboardUI`) ScoreTeam))

(event `Grab Ball`
  ;[1 1 1] Grab ball (no long grabbable)
  (`/Engine/EditorBlueprintResources/ActorMacros.Switch Has Authority`
    (:`Authority`
      (set `self.bIsGrabbable` false)
      (`KismetSystemLibrary.PrintString` (`KismetStringLibrary.Concat_StrStr` "Ball says:" "ball is grabbed")))))

(event `Release Ball`
  ;[1 1 1] Release Ball
  (`/Engine/EditorBlueprintResources/ActorMacros.Switch Has Authority`
    (:`Authority`
      (set `self.bIsGrabbable` true)
      (`KismetSystemLibrary.PrintString` (`KismetStringLibrary.Concat_StrStr` "Ball says:" "ball is released")))))

(event `Ball Shoot Ball`
  (params (ShotVelocity :type "Vector Structure"))
  (bind _staticmeshcomponent (`self.StaticMeshComponent`))
  (`/Engine/EditorBlueprintResources/ActorMacros.Switch Has Authority`
    (:`Authority`
      (`self.K2_DetachFromActor` "KeepWorld" "KeepWorld" "KeepWorld")
      (`PrimitiveComponent.SetSimulatePhysics` _staticmeshcomponent true)
      (`PrimitiveComponent.SetPhysicsLinearVelocity` _staticmeshcomponent ShotVelocity false "None")
      (`self.Release Ball`)
      (`self.SetActorEnableCollision` self true))))

(event `BallShootBall wRotation`
  (params (ShotVelocity :type "Vector Structure") (ShotRotationOffset :type "Float (double-precision)") (Shooter :type "Actor Object Reference"))
  (bind _staticmeshcomponent (`self.StaticMeshComponent`))
  (`self.K2_DetachFromActor` "KeepWorld" "KeepWorld" "KeepWorld")
  (`self.K2_SetActorLocation` (`KismetMathLibrary.RotateAngleAxis` (`self.K2_GetActorLocation`) ShotRotationOffset (`self.K2_GetActorLocation` Shooter)))
  (`PrimitiveComponent.SetSimulatePhysics` _staticmeshcomponent true)
  (`PrimitiveComponent.SetPhysicsLinearVelocity` _staticmeshcomponent ShotVelocity false "None")
  (`self.Release Ball`)
  (`self.SetActorEnableCollision` self true))

(fn `UserConstructionScript`)