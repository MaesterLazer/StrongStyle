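; Basketball hoop actor that tells the game camera when it becomes the active hoop.
; Shortly after BeginPlay it searches for camera actors and caches the BP_Camera_LOCAL as GameCamera.
; When an actor tagged Ball leaves the BallCameraCheck volume, roughly at midcourt, the hoop sets itself as that camera's ActiveHoop.
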(event `self.ReceiveBeginPlay`
  (`KismetSystemLibrary.Delay` 1.0)
  (bind _outactors (`GameplayStatics.GetAllActorsOfClass` (`self.GameCameraClass`)))
  (for _array_element _outactors
    (bind _asbp_camera_local (cast `/Game/BLUEPRINT/LOCAL/BP_Camera_LOCAL` _array_element))
    (set `self.GameCamera` _asbp_camera_local)))

(event `self.BallCameraCheck.OnComponentEndOverlap`
  (params (OverlappedComponent :type "PrimitiveComponent Object Reference") (OtherActor :type "Actor Object Reference") (OtherComp :type "PrimitiveComponent Object Reference") (OtherBodyIndex :type Integer))
  ;[1 1 1 1 28] Ball Camera check as crossing midcourtish
  (if (`self.ActorHasTag` OtherActor "Ball")
    (set `/Game/BLUEPRINT/LOCAL/BP_Camera_LOCAL.ActiveHoop` self (`self.GameCamera`))))

(fn `UserConstructionScript`)