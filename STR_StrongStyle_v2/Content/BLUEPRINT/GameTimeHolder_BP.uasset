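; GameTimeHolder_BP is a match clock holder for the basketball game, exposing MatchTime through GetMatchTime.
; On BeginPlay it binds to the player character's GameStart dispatcher, which records the start timestamp.
; Tick refreshes MatchTime from TimeElapsedSinceGameStart, whose graph holds only an unused countdown expression (time limit minus elapsed time).
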(event `self.ReceiveBeginPlay`
  ;[1 1 1] EVENTS
  ;[1 1 1] DISPATCH BIND: GameStart
  (bind _asbp_basketball_player_m (cast `/Game/BLUEPRINT/PLAYERS/BP_BasketballPlayer_M` (`GameplayStatics.GetPlayerCharacter` 0)))
  (add `/Game/BLUEPRINT/PLAYERS/BP_BasketballPlayer_M.Dispatcher_GameStart` _asbp_basketball_player_m (delegate `StartMatchClock`)))

(event `StartMatchClock`
  ;[1 1 1] EVENTS
  ;[1 1 1] Start Game Clock
  (set `self.GameStartTimestamp` (`KismetSystemLibrary.GetGameTimeInSeconds`))
  (set `self.GameTimeLimitSeconds` (`self.GameTimeLimitSeconds`)))

(event `self.ReceiveTick`
  (params (DeltaSeconds :type "Float (single-precision)"))
  ;[1 1 1] EVENTS
  (set `self.MatchTime` (`self.Time Elapsed Since Game Start`)))

(fn `Get Match Time`
  (returns (MatchTime :type "Float (double-precision)"))
  (return (`self.MatchTime`)))

(fn `UserConstructionScript`)