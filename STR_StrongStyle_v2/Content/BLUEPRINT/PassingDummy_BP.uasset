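; PassingDummy_BP is a dummy actor that picks up the ball on overlap.
; GrabBall takes the first overlapping actor as TheBall without a type check, disables its collision and physics, and attaches it to a hand socket.
; It then sets possession and shoot flags, and clears CanGrabBall to block further grabs.
; No passing, shooting or release logic is present.
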(event `self.ReceiveActorBeginOverlap`
  (params (OtherActor :type "Actor Object Reference"))
  ;[1 1 1] CUSTOM: Picking Up Ball
  (if (`self.CanGrabBall`)
    (`self.Grab Ball`)))

(fn `Grab Ball`
  (locals (NewLocalVar_0 :type "Actor Object Reference"))
  ;[1 1 1] Grab Ball
  (if (`self.CanGrabBall`)
    (set `self.CanGrabBall` false)
    (bind _output_get (set `self.GrabActorList` (`self.GetOverlappingActors` null)))
    (bind _output_get_2 (set `self.GrabbableBall` (`|GetArrayItem` _output_get)))
    (set `self.TheBall` _output_get_2) ; DO BETTER LATER When we pick the ball up, TheBall is defined.
    (`self.SetActorEnableCollision` _output_get_2 false)
    (bind _output_get_3 (set `self.BallInHands` (`self.GetComponentByClass` _output_get_2 "/Script/Engine.StaticMeshComponent")))
    (`PrimitiveComponent.SetSimulatePhysics` _output_get_3 false)
    (`self.K2_AttachToComponent` (`self.GrabbableBall`) (`self.StaticMeshComponent`) (`self.HandSocketName`) "SnapToTarget" "KeepRelative" "KeepRelative" false)
    (set `self.HasPosession` true)
    (set `self.CanShoot` true)))

(fn `UserConstructionScript`)