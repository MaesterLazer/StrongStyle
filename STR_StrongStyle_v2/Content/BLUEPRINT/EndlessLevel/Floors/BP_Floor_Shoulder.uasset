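; Floor shoulder Blueprint for the endless level that scatters instanced static meshes through a box volume.
; The construction script calls the parent, moves the instanced mesh component to the box's relative location as a world position, then rebuilds all instances.
; Each instance gets a random point within the box bounds and independently random X, Y and Z scales, with no random rotation.
; BeginPlay only calls the parent.
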(event `self.ReceiveBeginPlay`
  (`parent.ReceiveBeginPlay`))

(fn `UserConstructionScript`
  (bind _minxyscale (`self.MinXYScale`))
  (bind _maxxyscale (`self.MaxXYScale`))
  (bind (_origin _boxextent) (`KismetSystemLibrary.GetComponentBounds` (`self.Box`)))
  (`parent.UserConstructionScript`)
  (`SceneComponent.K2_SetWorldLocation` (`self.InstancedStaticMesh`) (`SceneComponent.RelativeLocation` (`self.Box`)) false false)
  (`InstancedStaticMeshComponent.ClearInstances` (`self.InstancedStaticMesh`))
  (for _ (range (+ (`self.NumberOfInstances`) 1))
    ;[1 1 1] Add instanced mesh of random scale to random location within bounding box
    (`InstancedStaticMeshComponent.AddInstance` (`self.InstancedStaticMesh`) (`KismetMathLibrary.MakeTransform` (`KismetMathLibrary.RandomPointInBoundingBox` _origin _boxextent) (struct) (`KismetMathLibrary.MakeVector` (`KismetMathLibrary.RandomFloatInRange` _minxyscale _maxxyscale) (`KismetMathLibrary.RandomFloatInRange` _minxyscale _maxxyscale) (`KismetMathLibrary.RandomFloatInRange` (`self.MinZScale`) (`self.MaxZScale`))))) ; Could randomize scale, but wont for now
  ))