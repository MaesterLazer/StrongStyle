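; Actor component that continuously scrolls its owning actor in the endless level.
; On BeginPlay it caches the EndlessLevelManager found through GetLevelManager.
; Each tick it scales the owner's forward vector by the manager's LevelSpeed and delta time for framerate-independent movement.
; That world-space vector is applied as a local offset without sweep, so the owner's rotation affects the direction twice.
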(event `self.ReceiveBeginPlay`
  (bind (_endlesslevelmanager _managerfound) (`/Game/BLUEPRINT/EndlessLevel/Lib/BPF_Lib.GetLevelManager`))
  (if _managerfound
    (set `self.LevelManagerRef` _endlesslevelmanager)))

(event `self.ReceiveTick`
  (params (DeltaSeconds :type "Float (single-precision)"))
  (set `self.DeltaSeconds` DeltaSeconds)
  (bind _output_get (set `self.Movement` (* (* (`Actor.GetActorForwardVector` (`self.GetOwner`)) (`/Game/BLUEPRINT/EndlessLevel/BP_EndlessLevelManager.LevelSpeed` (`self.LevelManagerRef`))) (`self.DeltaSeconds`))))
  (`Actor.K2_AddActorLocalOffset` (`self.GetOwner`) _output_get false false))