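; BP_Spawner_Floor is a child spawner that builds and recycles a row of floor tiles for an endless level.
; On BeginPlay it spawns the required count through the parent's SpawnActor, measures tile length from the first tile's X bounds and lays the rest end to end along +X.
; When a tile hits bounds, it is moved behind the tracked RearTile and becomes the new rear, avoiding respawns.
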(event `self.ReceiveBeginPlay`
  (bind (_returnvalue_x _returnvalue_y _returnvalue_z) (`KismetMathLibrary.BreakVector` (`self.K2_GetActorLocation` (`self.RearTile`))))
  (`parent.ReceiveBeginPlay`)
  (for _index (range (`self.ActorRequiredCount`))
    ;[1 1 1] Check if first one spawned
    (if (== _index 0)
      ;[1 1 1] First Tile Spawning
      (bind _spawnedactor (`self.SpawnActor`))
      (set `self.RearTile` _spawnedactor)
      (set `self.TileSize` (* (.x (`.BoxExtent` (`self.GetActorBounds` _spawnedactor false))) 2.0))
      (`self.K2_SetActorLocation` (`self.RearTile`) (`self.K2_GetActorLocation`) false false)
      (else
        (bind _spawnedactor_2 (`self.SpawnActor`))
        (`self.K2_SetActorLocation` _spawnedactor_2 (`KismetMathLibrary.MakeVector` (+ (`self.TileSize`) _returnvalue_x) _returnvalue_y _returnvalue_z) false false)
        (set `self.RearTile` _spawnedactor_2)))))

(event `self.SpawnActorHitBounds`
  (params (OutOfBoundsActor :type "Actor Object Reference"))
  (bind (_returnvalue_x _returnvalue_y _returnvalue_z) (`KismetMathLibrary.BreakVector` (`self.K2_GetActorLocation` (`self.RearTile`))))
  (`self.K2_SetActorLocation` OutOfBoundsActor (`KismetMathLibrary.MakeVector` (+ (`self.TileSize`) _returnvalue_x) _returnvalue_y _returnvalue_z) false false)
  (set `self.RearTile` OutOfBoundsActor))

(fn `SpawnActor`
  (returns (SpawnedActor :type "Actor Object Reference"))
  (bind _spawnedactor (`parent.SpawnActor`))
  (return _spawnedactor))

(fn `UserConstructionScript`
  (`parent.UserConstructionScript`))