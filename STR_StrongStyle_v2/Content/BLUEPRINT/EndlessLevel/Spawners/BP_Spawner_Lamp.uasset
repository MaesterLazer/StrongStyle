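; Spawner for an endless level that lines up a row of lamps along X and recycles them, extending a parent spawner class.
; On BeginPlay it spawns the required count from its own location, turning lamps 180 degrees for a right-side spawner.
; Spacing comes from the first lamp's X bounds scaled by an offset.
; When a lamp hits bounds, it moves one spacing past the tracked rear lamp and becomes the new rear, avoiding respawns.
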(event `self.ReceiveBeginPlay`
  (bind (_returnvalue_x _returnvalue_y _returnvalue_z) (`KismetMathLibrary.BreakVector` (`self.K2_GetActorLocation` (`self.RearLamp`))))
  (`parent.ReceiveBeginPlay`)
  (if (`self.IsRightSideSpawner`)
    (set `self.LampRotation` (struct :`Yaw` 180.0))
    (else
      (set `self.LampRotation` (struct))))
  (for _index (range (`self.ActorRequiredCount`))
    ;[1 1 1] Check if first one spawned
    (if (== _index 0)
      ;[1 1 1] First Tile Spawning
      (bind _spawnedactor (`self.SpawnActor`))
      (set `self.RearLamp` _spawnedactor)
      (set `self.LampSize` (* (.x (`.BoxExtent` (`self.GetActorBounds` _spawnedactor false))) (`self.LampOffset`)))
      (`self.K2_SetActorLocationAndRotation` (`self.RearLamp`) (`self.K2_GetActorLocation`) (`self.LampRotation`) false false)
      (else
        (bind _spawnedactor_2 (`self.SpawnActor`))
        (`self.K2_SetActorLocationAndRotation` _spawnedactor_2 (`KismetMathLibrary.MakeVector` (+ (`self.LampSize`) _returnvalue_x) _returnvalue_y _returnvalue_z) (`self.LampRotation`) false false)
        (set `self.RearLamp` _spawnedactor_2)))))

(event `self.SpawnActorHitBounds`
  (params (OutOfBoundsActor :type "Actor Object Reference"))
  (bind (_returnvalue_x _returnvalue_y _returnvalue_z) (`KismetMathLibrary.BreakVector` (`self.K2_GetActorLocation` (`self.RearLamp`))))
  (`self.K2_SetActorLocation` OutOfBoundsActor (`KismetMathLibrary.MakeVector` (+ (`self.LampSize`) _returnvalue_x) _returnvalue_y _returnvalue_z) false false)
  (set `self.RearLamp` OutOfBoundsActor))

(fn `SpawnActor`
  (returns (SpawnedActor :type "Actor Object Reference"))
  (bind _spawnedactor (`parent.SpawnActor`))
  (return _spawnedactor))

(fn `UserConstructionScript`
  (`parent.UserConstructionScript`))