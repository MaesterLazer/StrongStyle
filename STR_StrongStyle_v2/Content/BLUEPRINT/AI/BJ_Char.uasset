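; AI basketball character that acts as a shot blocker against the local player.
; On BeginPlay it writes an AI_MoveTo actor to its blackboard as Target and caches the player character.
; Tick polls the player's IsShooting flag, jumping with the block mesh visible and collidable while true, hiding it otherwise.
; Functions handle team 2 registration with the game mode, including the offense hoop, and a delay-based stun.
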(event `self.ReceiveBeginPlay`
  ;[1 1 1] Set Target
  (bind _outactors (`GameplayStatics.GetAllActorsOfClass` "/Script/STR_StrongStyle_v2.AI_MoveTo"))
  (for _array_element _outactors
    (set `self.Target` _array_element))
  ;[1 1 1] Set Blackboard Target
  (`BlackboardComponent.SetValueAsObject` (`AIBlueprintHelperLibrary.GetBlackboard` (`AIBlueprintHelperLibrary.GetAIController` self)) "Target" (`self.Target`))
  ;[1 1 1] Set Player
  (bind _asbp_basketball_player_local (cast `/Game/BLUEPRINT/LOCAL/BP_BasketballPlayer_Local` (`GameplayStatics.GetPlayerCharacter` 0)))
  (set `self.Player` _asbp_basketball_player_local))

(event `self.ReceiveTick`
  (params (DeltaSeconds :type "Float (single-precision)"))
  (bind _blocknormalmesh (`self.BlockNormalMesh`))
  (bind _blocknormalmesh_2 (`self.BlockNormalMesh`))
  (if (`/Game/BLUEPRINT/LOCAL/BP_BasketballPlayer_Local.isShooting` (`self.Player`))
    (`PrimitiveComponent.SetCollisionEnabled` _blocknormalmesh_2 "QueryAndPhysics")
    (`SceneComponent.SetVisibility` _blocknormalmesh_2 true false)
    (set `CharacterMovementComponent.JumpZVelocity` 575.0 (`self.CharacterMovement`))
    (`self.Jump`)
    (else
      (`PrimitiveComponent.SetCollisionEnabled` _blocknormalmesh "NoCollision")
      (`SceneComponent.SetVisibility` _blocknormalmesh false false))))

(event `Event StunCooldown`
  (params (StunCooldownTime :type "Float (double-precision)"))
  ;[1 1 1] Get Stunned
  (`KismetSystemLibrary.Delay` StunCooldownTime)
  (set `self.bIsStunned` false))

(fn `BecomeStunned`
  (params (StunCooldownTime :type "Float (double-precision)"))
  (set `self.bIsStunned` true)
  (`self.Event StunCooldown` StunCooldownTime))

(fn `SetTeam2`
  (bind _returnvalue (`GameplayStatics.GetGameMode`))
  ;[1 1 1] Add to Team 1 in Game Mode
  (set `self.MyTeam` 2)
  (bind _asbasket_ball_game_mode_local (cast `/Game/BLUEPRINT/LOCAL/BasketBallGameMode_Local` _returnvalue))
  (`KismetArrayLibrary.Array_Add` (`/Game/BLUEPRINT/LOCAL/BasketBallGameMode_Local.TeamPlayers2` _asbasket_ball_game_mode_local) self)
  ;[1 1 1] Remove from Team 2 in Game Mode
  (bind _asbasket_ball_game_mode_local_2 (cast `/Game/BLUEPRINT/LOCAL/BasketBallGameMode_Local` _returnvalue))
  (`KismetArrayLibrary.Array_RemoveItem` (`/Game/BLUEPRINT/LOCAL/BasketBallGameMode_Local.TeamPlayers1` _asbasket_ball_game_mode_local_2))
  ;[1 1 1] Set target hoop
  (bind _asbasket_ball_game_mode_local_3 (cast `/Game/BLUEPRINT/LOCAL/BasketBallGameMode_Local` (`GameplayStatics.GetGameMode`)))
  (set `self.HoopOffense` (`/Game/BLUEPRINT/LOCAL/BasketBallGameMode_Local.HoopTeam1` _asbasket_ball_game_mode_local_3)))

(fn `UserConstructionScript`)