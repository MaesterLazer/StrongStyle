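; BJ_AI is an AI-controlled actor that targets whichever basketball player has possession of the ball.
; On BeginPlay it caches all BP_BasketballPlayer_Local actors, then checks their HasPosession flags every Tick.
; The possessing player is written to the PlayerObj blackboard key, with player character 0 as fallback.
; A NoPossess flag, reset each frame, decides when that fallback applies.
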(event `self.ReceiveBeginPlay`
  (bind _outactors (`GameplayStatics.GetAllActorsOfClass` "/Game/BLUEPRINT/LOCAL/BP_BasketballPlayer_Local.BP_BasketballPlayer_Local_C"))
  (set `self.Players` _outactors))

(event `self.ReceiveTick`
  (params (DeltaSeconds :type "Float (single-precision)"))
  (for _array_element (`self.Players`)
    (if (`/Game/BLUEPRINT/LOCAL/BP_BasketballPlayer_Local.bHasPosession` _array_element)
      (bind _output_get (set `self.Target` _array_element))
      (`BlackboardComponent.SetValueAsObject` (`AIBlueprintHelperLibrary.GetBlackboard` (`AIBlueprintHelperLibrary.GetAIController` self)) "PlayerObj" _output_get)
      (set `self.noPossess` false)))
  (if (`self.noPossess`)
    (bind _output_get_2 (set `self.Target` (`GameplayStatics.GetPlayerCharacter` 0)))
    (`BlackboardComponent.SetValueAsObject` (`AIBlueprintHelperLibrary.GetBlackboard` (`AIBlueprintHelperLibrary.GetAIController` self)) "PlayerObj" _output_get_2)
    (set `self.noPossess` true)
    (else
      (set `self.noPossess` true))))

(fn `UserConstructionScript`)