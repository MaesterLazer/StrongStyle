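; Game instance for local play that puts the main UI widgets on screen.
; AddWidgetPause creates BPW_MenuMain as the pause menu, shows the cursor and switches player 0 to game-and-UI input focused on it.
; AddWidgetUI creates the in-game UI widget and stores it as ScoreboardUI.
; GameInstanceLocalCameraSetup is a defunct empty event, with its old loop over BP_Camera_v2 initial setup left disconnected.
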(event `AddWidgetPause`
  (bind _returnvalue (`GameplayStatics.GetPlayerController` 0))
  ;[1 1 1] Pause Menu
  (bind _returnvalue_2 (`|CreateWidget` "/Game/BLUEPRINT/WIDGETS/BPW_MenuMain.BPW_MenuMain_C" _returnvalue))
  (`UserWidget.AddToViewport` _returnvalue_2 0)
  (set `PlayerController.bShowMouseCursor` true _returnvalue)
  (`WidgetBlueprintLibrary.SetInputMode_GameAndUIEx` _returnvalue _returnvalue_2))

(event `AddWidgetUI`
  ;[1 1 1] Pause Menu
  ;;[1 1 1] Add UI
  (bind _returnvalue (`|CreateWidget` "/Game/BLUEPRINT/WIDGETS/BPW_InGameUI.BPW_InGameUI_C"))
  (bind _output_get (set `self.ScoreboardUI` _returnvalue))
  (`UserWidget.AddToViewport` _output_get 0))

(event `Event GameInstance LocalCameraSetup`
  ;[1 1 1] DEFUNCT Local Camera Class Setup (Get Players)
)