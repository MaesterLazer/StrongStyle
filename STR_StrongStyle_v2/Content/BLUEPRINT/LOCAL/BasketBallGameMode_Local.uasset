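; Game mode for local multiplayer basketball that sets up the match when the level begins play.
; A one-time startup finds tagged hoops by team, creates and possesses a player at each index-tagged PlayerStart, alternates team changes, and spawns the ball.
; It broadcasts offense phase updates to all tagged players, starting with placeholder team 3.
; Helper events maintain team arrays and forward player refreshes to the GameState; older UI and player-creation logic is disconnected.
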(event `self.ReceiveBeginPlay`
  ;[1 1 1] BEGIN PLAY (Nothing)
  (`self.Event Startup`))

(event `Event Startup`
  ;[1 1 1] STARTUP ON LOAD LEVEL
  (`/Engine/EditorBlueprintResources/StandardMacros.DoOnce` false
    (:`Completed`
      (`KismetSystemLibrary.PrintString` "GAMEMODE > ON HOST LEVEL CALLED, STARTING GAMEMODE" true true (struct :`R` 1.0 :`G` 0.9302 :`A` 1.0) (`self.DebugDuration`))
      ;;[1 1 1] Populate Hoops Array and Set Team Hoops
      (`self.PopulateHoops`)
      (`self.SetHoops`)
      ;;[1 1 1] Get Spawnpoints, Spawn Players
      (`self.GetPlayerStartPoints`)
      ;;[1 1 1] Local Game Player Spawn
      (`KismetSystemLibrary.PrintString` "GAMEMODE > LOCAL GAME DETECTED, SPAWNING PLAYERS" true true (`self.DebugColor`) (`self.DebugDuration`))
      (`self.SpawnPlayers`)
      ;;[1 1 1] SpawnBall
      (`self.SpawnBall` null)
      ;;[1 1 1] Initial Phase Assignment
      (`self.Event UpdateAllPhaseAssignments` 3 true) ; Team3 b/c even w/ spectators, there should never be a Team 3
    )))

(event `EventGM RefreshPlayers`
  ;[1 1 1] GameState Refresh Players Array
  (`KismetSystemLibrary.PrintString` "GAMEMODE > CALLING GAMESTATE (REFRESH PLAYERS)" true true (`self.DebugColor`) (`self.DebugDuration`))
  (bind _asbp_game_state_local (cast `/Game/BLUEPRINT/LOCAL/BP_GameState_Local` (`GameplayStatics.GetGameState`)))
  (`/Game/BLUEPRINT/LOCAL/BP_GameState_Local.EventGS RefreshPlayers` _asbp_game_state_local))

(event `self.K2_PostLogin`
  (params (NewPlayer :type "PlayerController Object Reference"))
  ;[1 1 1] Post Login
  (`KismetSystemLibrary.PrintString` (`KismetStringLibrary.Concat_StrStr` "GAMEMODE > POST LOGIN: " (`KismetSystemLibrary.GetDisplayName` NewPlayer) "has joined!") true true (`self.DebugColor`) (`self.DebugDuration`)))

(event `Event UpdateAllPhaseAssignments`
  (params (OffenseTeam :type Integer) (bBallReleaseNoTeam :type Boolean))
  ;[1 1 1] Phase Assignment/Update (Triggered by picking up ball)
  (bind _outactors (`GameplayStatics.GetAllActorsWithTag` "Player"))
  (for _array_element _outactors
    (bind _asbp_basketball_player_local (cast `/Game/BLUEPRINT/LOCAL/BP_BasketballPlayer_Local` _array_element)
      (:`then`
        (`/Game/BLUEPRINT/LOCAL/BP_BasketballPlayer_Local.Event UpdatePhaseAssignment` _asbp_basketball_player_local OffenseTeam bBallReleaseNoTeam))
      (:`CastFailed`
        (`KismetSystemLibrary.PrintString` "GAMEMODE x PHASE ASSIGNMENT PLAYER CAST FAILED"))))
  (`KismetSystemLibrary.PrintString` "GAMEMODE > PHASE UPDATE COMPLETE"))

(event `PopulateHoops`
  ;[1 1 1] Populate Hoop Array
  (`self.PopulateHoopArray`))

(event `SetHoops`
  ;[1 1 1] Set Team Hoops
  (for _array_element (`self.GameHoops`)
    (bind _ashoop_bp (cast `/Game/BLUEPRINT/Hoop_BP` _array_element))
    (bind _hoopteam (`/Game/BLUEPRINT/Hoop_BP.HoopTeam` _ashoop_bp))
    (if (== _hoopteam 1)
      (set `self.HoopTeam1` _array_element)
      (elif (== _hoopteam 2)
        (set `self.HoopTeam2` _array_element))))
  (`KismetSystemLibrary.PrintString` "GAMEMODE > HOOPS SET" true true (`self.DebugColor`) (`self.DebugDuration`)))

(event `PopulateTeamArrays`
  ;[1 1 1] Populate Team Arrays
  (bind _outactors (`GameplayStatics.GetAllActorsWithTag` "Player"))
  (for _array_element _outactors
    (bind _asbp_basketball_player_local (cast `/Game/BLUEPRINT/LOCAL/BP_BasketballPlayer_Local` _array_element)
      (:`then`
        (bind _myteam (`/Game/BLUEPRINT/LOCAL/BP_BasketballPlayer_Local.MyTeam` _asbp_basketball_player_local))
        (if (== _myteam 1)
          (`KismetArrayLibrary.Array_Add` (`self.TeamPlayers1`) _array_element)
          (elif (== _myteam 2)
            (`KismetArrayLibrary.Array_Add` (`self.TeamPlayers2`) _array_element))))
      (:`CastFailed`
        ;[1 1 1] Fail
        (`KismetSystemLibrary.PrintString` "GAMEMODE x POPULATE TEAM ARRAY PLAYER CAST FAILED!" true true (`self.DebugColorFAILED`) (`self.DebugDuration`))))))

(event `ClearTeamArrays`
  ;[1 1 1] Clear Team Arrays
  (`KismetArrayLibrary.Array_Clear` (`self.TeamPlayers1`))
  (`KismetArrayLibrary.Array_Clear` (`self.TeamPlayers2`)))

(fn `GetPlayerStartPoints`
  (bind _outactors (`GameplayStatics.GetAllActorsOfClass` "/Script/Engine.PlayerStart"))
  (set `self.PlayerStartArray` _outactors)
  (`KismetSystemLibrary.PrintString` "GAMEMODE > PLAYER START POINTS ACQUIRED" true true (`self.DebugColor`) (`self.DebugDuration`)))

(fn `PopulateHoopArray`
  (returns (Output_Get :type "Array of Actor Object Reference"))
  ;[1 1 1] Populate Hoop Array
  (bind _outactors (`GameplayStatics.GetAllActorsWithTag` "Hoop"))
  (bind _output_get (set `self.GameHoops` _outactors))
  (`KismetSystemLibrary.PrintString` "GAMEMODE > HOOPS POPULATED" true true (`self.DebugColor`) (`self.DebugDuration`))
  (return _output_get))

(fn `SetBallUIRef`
  (params (self2 :type "/Game/BLUEPRINT/LOCAL/Ball_BP Object Reference"))
  (set `/Game/BLUEPRINT/LOCAL/Ball_BP.ScoreboardUI` (`self.ScoreboardUI`) (`self.GameBall`)))

(fn `SetScoreboardUI`
  (params (ScoreboardUISet :type "/Game/BLUEPRINT/WIDGETS/BPW_InGameUI Object Reference"))
  (set `self.ScoreboardUI` ScoreboardUISet))

(fn `SetTeamHoops`
  (params (Array :type "Array of Actor Object Reference"))
  ;[1 1 1] Set Team Hoops
  (for _array_element Array
    (bind _ashoop_bp (cast `/Game/BLUEPRINT/Hoop_BP` _array_element))
    (bind _hoopteam (`/Game/BLUEPRINT/Hoop_BP.HoopTeam` _ashoop_bp))
    (if (== _hoopteam 1)
      (set `self.HoopTeam1` _ashoop_bp)
      (elif (== _hoopteam 2)
        (set `self.HoopTeam2` _ashoop_bp)))))

(fn `SpawnBall`
  (params (InputPin :type "/Game/BLUEPRINT/WIDGETS/BPW_InGameUI Object Reference"))
  (`KismetSystemLibrary.PrintString` "GAMEMODE > SPAWNING BALL" true true (`self.DebugColor`) (`self.DebugDuration`))
  ;[1 1 1] Spawn Ball
  (bind _returnvalue (`|SpawnActorFromClass` (`self.BallClass`) (`self.BallSpawnPoint`) "Undefined" "OverrideRootScale" null null))
  ;[1 1 1] Set Ball Ref for UI and Add to Viewport
  (bind _asball_bp (cast `/Game/BLUEPRINT/LOCAL/Ball_BP` _returnvalue))
  (set `self.GameBall` _asball_bp))

(fn `SpawnPlayers`
  (bind _index (`self.Index`))
  ;[1 1 1] Loop through max player index
  (for _index_2 (range (`self.MaxPlayerCount`))
    (set `self.Index` _index_2)
    ;[1 1 1] Find next Spawn Point, Create Player, and Spawn
    (for _array_element (`self.PlayerStartArray`)
      (if (== (`PlayerStart.PlayerStartTag` _array_element) (`KismetStringLibrary.Conv_StringToName` (`KismetStringLibrary.Conv_IntToString` (`self.Index`))))
        ;;[1 1 1] Create Player and Spawn PlayerBP
        (`GameplayStatics.CreatePlayer` (`self.Index`))
        (`KismetSystemLibrary.PrintString` (`KismetStringLibrary.Concat_StrStr` "GAMEMODE > CREATING PLAYER: for ID " (`KismetStringLibrary.Conv_IntToString` (`self.Index`))) true true (`self.DebugColor`) (`self.DebugDuration`))
        (bind _returnvalue (`|SpawnActorFromClass` "/Game/BLUEPRINT/LOCAL/BP_BasketballPlayer_Local.BP_BasketballPlayer_Local_C" (`self.GetTransform` _array_element) "Undefined" "OverrideRootScale" null null null))
        ;[1 1 1] Possess Spawned
        (`KismetSystemLibrary.PrintString` (`KismetStringLibrary.Concat_StrStr` "GAMEMODE > POSSESSING PLAYER:" "ID " (`KismetStringLibrary.Conv_IntToString` _index)) true true (`self.DebugColor`) (`self.DebugDuration`))
        (`Controller.Possess` (`GameplayStatics.GetPlayerController` _index) _returnvalue)
        ;[1 1 1] Change Teams so team sets
        (`/Engine/EditorBlueprintResources/StandardMacros.FlipFlop`
          (:`A`
            (`/Game/BLUEPRINT/LOCAL/BP_BasketballPlayer_Local.ChangeTeams` _returnvalue)
            (`/Game/BLUEPRINT/LOCAL/BP_BasketballPlayer_Local.ChangeTeams` _returnvalue))
          (:`B`
            (`/Game/BLUEPRINT/LOCAL/BP_BasketballPlayer_Local.ChangeTeams` _returnvalue)))))))

(fn `UserConstructionScript`)