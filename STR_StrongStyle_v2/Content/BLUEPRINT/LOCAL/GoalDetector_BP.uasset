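; GoalDetector_BP is a goal detector tied to a team's hoop, exposing that team and whether a score can currently count.
; SetScoreFalse clears the CanScore flag and starts ResetScoreTimer, which restores it after a short delay, forming a scoring cooldown.
; GetTeam and GetScore are plain getters for TeamHoop and CanScore; the file itself contains no overlap or scoring logic.
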(event `ResetScoreTimer`
  (`KismetSystemLibrary.Delay` 1.0)
  (set `self.bCanScore` true))

(event `SetScoreFalse`
  (set `self.bCanScore` false)
  (`self.ResetScoreTimer`))

(fn `Get Team`
  (returns (TeamNumber :type Integer))
  (return (`self.TeamHoop`)))

(fn `GetScore`
  (returns (bCanScore :type Boolean))
  (return (`self.bCanScore`)))

(fn `UserConstructionScript`)