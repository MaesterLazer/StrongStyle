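; Basketball actor that handles grab, release, shot, pass and steal launches, bounce sounds and scoring.
; Launches set physics velocity, raising weak passes to a minimum horizontal speed; optional homing redirects velocity toward a target each tick until hit or grab.
; Authority-checked grabs record the last team, and grabs and releases update GameMode phases.
; Leaving a goal detector awards 2, 3 or 4 points by shot distance through the GameInstance's scoreboard.
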(event `self.ReceiveTick`
  (params (DeltaSeconds :type "Float (single-precision)"))
  ;[1 1 1] TICK + HOMING
  (if (`self.bIsHoming`)
    (`self.Event Homing`)))

(event `EventStatus Homing`
  (params (HomingTarget :type "Actor Object Reference"))
  ;[1 1 1] STATUS AND COLLISION "STATES"
  (set `self.HomingTarget` HomingTarget)
  (set `self.bIsHoming` true))

(event `EventOnline BallLaunch`
  (params (`Shot Velocity` :type "Vector Structure") (Target :type "Actor Object Reference") (Homing :type Boolean) (HomingTarget :type "Actor Object Reference") (Pass :type Boolean))
  ;[1 1 1 1 28] Local Ball Launch
  (`self.EventLocal BallLaunch` Target `Shot Velocity` Pass false Homing null HomingTarget))

(event `self.ReceiveBeginPlay`
  ;[1 1 1] Add UI and set Reference
  (bind _asbp_game_instance (cast `/Game/BLUEPRINT/BP_GameInstance` (`GameplayStatics.GetGameInstance`))
    (:`then`
      (`/Game/BLUEPRINT/BP_GameInstance.AddWidgetUI` _asbp_game_instance)
      (set `self.ScoreboardUI` (`/Game/BLUEPRINT/BP_GameInstance.ScoreboardUI` _asbp_game_instance)))
    (:`CastFailed`
      (`KismetSystemLibrary.PrintString` "Ball Game Instance Cast Failed!"))))

(event `self.StaticMeshComponent.OnComponentHit`
  (params (HitComponent :type "PrimitiveComponent Object Reference") (OtherActor :type "Actor Object Reference") (OtherComp :type "PrimitiveComponent Object Reference") (NormalImpulse :type "Vector Structure") (Hit :type "HitResult Structure (by ref)"))
  ;[1 1 1] BOUNCE EFFECTS
  (if (`self.bIsHoming`)
    (`self.EventStatus StopHoming`))
  (if (`self.bCanBounceSFX`)
    (`self.SFX Bounce` Hit OtherActor)))

(event `self.ReceiveActorBeginOverlap`
  (params (OtherActor :type "Actor Object Reference"))
  ;[1 1 1] Scoring
  ;;[1 1 1] Player/Goal Check
  (if (`self.ActorHasTag` OtherActor "Player")
    _))

(event `EventStatus ReleaseBall`
  ;[1 1 1] STATUS AND COLLISION "STATES"
  (set `self.bIsGrabbable` true)
  (`self.K2_DetachFromActor` "KeepWorld" "KeepWorld" "KeepWorld")
  (`PrimitiveComponent.SetCollisionProfileName` (`self.StaticMeshComponent`) "CustomBall")
  (`PrimitiveComponent.SetSimulatePhysics` (`self.StaticMeshComponent`) true))

(event `self.ReceiveActorEndOverlap`
  (params (OtherActor :type "Actor Object Reference"))
  ;[1 1 1] Scoring
  ;;[1 1 1] Player/Goal Check
  (if (`self.ActorHasTag` OtherActor "GoalDetector")
    (`self.ScoreBasket` OtherActor)))

(event `EventStatus BallGrabbed`
  ;[1 1 1] STATUS AND COLLISION "STATES"
  ;;[1 1 1 1 28] Status: Ball Grabbed
  (set `self.bIsGrabbable` false)
  (`self.EventStatus StopHoming`)
  (`self.Reset SFX Bounce`)
  ;;[1 1 1] Start initial clock
  (`/Engine/EditorBlueprintResources/StandardMacros.DoOnce` false
    (:`Completed`
      (`/Game/BLUEPRINT/WIDGETS/BPW_InGameUI.ResetTime` (`self.ScoreboardUI`)))))

(event `EventLocal BallLaunch`
  (params (Target :type "Actor Object Reference") (Velocity :type "Vector Structure") (bPass :type Boolean) (bSteal :type Boolean :default false) (bHoming :type Boolean) (StealVictim :type "Actor Object Reference") (HomingTarget :type "Actor Object Reference") (DistanceToHoop :type "Float (double-precision)"))
  (bind _staticmeshcomponent (`self.StaticMeshComponent`))
  ;[1 1 1 1 28] Local Ball Launch
  (if bPass
    (bind (_underminvelocity _clampvelocity) (`self.CheckPassVelocityMinMax` Velocity (`self.PassMinVel`)))
    (if _underminvelocity
      (`PrimitiveComponent.SetPhysicsLinearVelocity` _staticmeshcomponent _clampvelocity false "None")
      (else
        (`PrimitiveComponent.SetPhysicsLinearVelocity` _staticmeshcomponent Velocity false "None" :!label _label)))
    (elif bSteal
      (bind _asbp_basketball_player_local (cast `/Game/BLUEPRINT/LOCAL/BP_BasketballPlayer_Local` StealVictim))
      (`/Game/BLUEPRINT/LOCAL/BP_BasketballPlayer_Local.EventStatus StealVictim` _asbp_basketball_player_local)
      (goto _label)
      (else
        (set `self.ScoreDistance` DistanceToHoop) ; ForPointCalculation
        (goto _label))))
  (`self.LOCAL ReleaseBall`)
  (`self.Event BallCallGMPhaseUpdate` 0 true)
  (if bHoming
    (`self.EventStatus Homing` HomingTarget)))

(event `ScoreBasket`
  (params (GoalDetector :type "Object Object Reference"))
  ;[1 1 1] Scoring
  ;;[1 1 1] Score Basket
  (`/Engine/EditorBlueprintResources/ActorMacros.Switch Has Authority`
    (:`Authority`
      (bind _asgoal_detector_bp (cast `/Game/BLUEPRINT/LOCAL/GoalDetector_BP` GoalDetector))
      (bind _bcanscore (`/Game/BLUEPRINT/LOCAL/GoalDetector_BP.GetScore` _asgoal_detector_bp))
      (if _bcanscore
        (`/Game/BLUEPRINT/LOCAL/GoalDetector_BP.ResetScoreTimer` _asgoal_detector_bp) ; Prevent double goals
        (`self.UpdateScore` (`self.LastTeamTouch`))))))

(event `SFX Bounce`
  (params (Hit :type "HitResult Structure (by ref)") (HitActor :type "Actor Object Reference"))
  ;[1 1 1] BOUNCE EFFECTS
  ;;[1 1 1] Premeeting Quick adds: SFX
  (if (`self.ActorHasTag` HitActor "BounceSFX")
    (`/Engine/EditorBlueprintResources/StandardMacros.Do N` 5 :!label _label_2
      (:`Exit`
        (`GameplayStatics.PlaySound2D` (`self.SfxBounceGround`) (`KismetMathLibrary.RandomFloatInRange` 0.7 1.0) 1.0 0.0 null null)
        (set `self.bCanBounceSFX` false)
        (`self.Cooldown SFX Bounce`)))))

(event `Reset SFX Bounce`
  ;[1 1 1] BOUNCE EFFECTS
  ;;[1 1 1] Premeeting Quick adds: SFX
  (set `self.bCanBounceSFX` true)
  (goto _label_2 :!via `Reset`))

(event `EventStatus StopHoming`
  ;[1 1 1] STATUS AND COLLISION "STATES"
  ;;[1 1 1 1 28] Stop Homing
  (set `self.bIsHoming` false)
  (`KismetSystemLibrary.PrintString` "BALL > STOPPING HOMING"))

(event `UpdateScore`
  (params (ScoringTeam :type Integer))
  (bind _scoredistance (`self.ScoreDistance`))
  ;[1 1 1] Scoring
  ;;[1 1 1] Update Score
  (if (<= _scoredistance (`self.3PointMaxDist`))
    (if (<= _scoredistance (`self.2PointMaxDist`))
      (set `self.ScoreValue` 2)
      (else
        (set `self.ScoreValue` 3)))
    (else
      (set `self.ScoreValue` 4)))
  (`/Game/BLUEPRINT/WIDGETS/BPW_InGameUI.UpdateScore` (`self.ScoreboardUI`) ScoringTeam (`self.ScoreValue`)))

(event `Cooldown SFX Bounce`
  ;[1 1 1] BOUNCE EFFECTS
  ;;[1 1 1] Premeeting Quick adds: SFX
  (`KismetSystemLibrary.Delay` (`self.CooldownTimeSFXBounce`))
  (set `self.bCanBounceSFX` true))

(event `LOCAL ReleaseBall`
  ;[1 1 1 1 28] Local Release Ball
  (`self.EventStatus ReleaseBall`))

(event `Event Homing`
  ;[1 1 1 1 28] Homing
  (`PrimitiveComponent.SetPhysicsLinearVelocity` (`self.StaticMeshComponent`) (* (`KismetMathLibrary.GetForwardVector` (`KismetMathLibrary.FindLookAtRotation` (`SceneComponent.K2_GetComponentLocation` (`self.StaticMeshComponent`)) (`self.K2_GetActorLocation` (`self.HomingTarget`)))) (`KismetMathLibrary.VSize` (`self.GetVelocity` self))) false "None"))

(event `Event BallGrabBall`
  (params (GrabberTeam :type Integer))
  ;[1 1 1] Grab ball (no long grabbable)
  (`/Engine/EditorBlueprintResources/ActorMacros.Switch Has Authority`
    (:`Authority`
      (`self.EventStatus BallGrabbed`)
      (bind _output_get (set `self.LastTeamTouch` GrabberTeam))
      (`self.Event BallCallGMPhaseUpdate` _output_get))))

(event `Event BallCallGMPhaseUpdate`
  (params (OffenseTeam :type Integer) (bBallReleaseNoTeam :type Boolean))
  ;[1 1 1] Call GM Phase Update
  (bind _asbasket_ball_game_mode_local (cast `/Game/BLUEPRINT/LOCAL/BasketBallGameMode_Local` (`GameplayStatics.GetGameMode`))
    (:`then`
      (`/Game/BLUEPRINT/LOCAL/BasketBallGameMode_Local.Event UpdateAllPhaseAssignments` _asbasket_ball_game_mode_local OffenseTeam bBallReleaseNoTeam))
    (:`CastFailed`
      (`KismetSystemLibrary.PrintString` "BALL x GM PHASE CAST FAILED"))))

(event `ONLINE ReleaseBall`
  ;[1 1 1] ONLINE Release Ball
  (`/Engine/EditorBlueprintResources/ActorMacros.Switch Has Authority`
    (:`Authority`
      (`self.LOCAL ReleaseBall`))))

(fn `CheckPassVelocityMinMax`
  (params (PassVector :type "Vector Structure") (PassMinimumVelocity :type "Float (double-precision)"))
  (returns (UnderMinVelocity :type Boolean) (ClampVelocity :type "Vector Structure"))
  (bind _returnvalue (`KismetMathLibrary.MakeVector` (.x PassVector) (.y PassVector)))
  (bind _returnvalue_2 (/ (`KismetMathLibrary.VSize` _returnvalue) PassMinimumVelocity))
  ;[1 1 1] BALL FORCES (Launch/Homing)
  (return (< _returnvalue_2 1.0) (`KismetMathLibrary.MakeVector` (.x (/ _returnvalue _returnvalue_2)) (.y (/ _returnvalue _returnvalue_2)) (.z PassVector))))

(fn `UserConstructionScript`)