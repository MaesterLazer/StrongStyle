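; Shared camera for the basketball game that follows and frames one to six players.
; After a short BeginPlay delay, ClassSetup reads players from BasketBallGameMode and sets this camera as the PlayerControllers' view target.
; A looping 0.001-second timer runs UpdateCamera, which picks per-player-count functions.
; These set spring arm length from the clamped largest pairwise distance and interpolate the actor toward the players' average position.
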(event `self.ReceiveBeginPlay`
  (`KismetSystemLibrary.Delay` 0.01)
  ;[1 1 1] TODO!!!: This needs to happen after spawn!
  (`self.ClassSetup`)
  (`KismetSystemLibrary.K2_SetTimer` null "UpdateCamera" 0.001 true) ; Refreshing less than tick (.001)
)

(event `CameraClassSetup`)

(event `UpdateCamera`
  ;[1 1 1] Adjust Arm Lengths based on Player Numbers
  (switch `int` (`KismetArrayLibrary.Array_Length` (`self.PlayersReference`))
    (:`1`
      (`self.SetArmLengthPlayers1`)
      ;[1 1 1] Set Camera Position and Lerp
      (`self.SetCameraPosPlayers1`))
    (:`2`
      (`self.SetArmLengthPlayers2`)
      (`self.SetCameraPosPlayers2`))
    (:`3`
      (`self.SetArmLengthPlayers3`)
      (`self.SetCameraPosPlayers3`))
    (:`4`
      (`self.SetArmLengthPlayers4`)
      (`self.SetCameraPosPlayers4`))
    (:`5`
      (`self.SetArmLengthPlayers5`)
      (`self.SetCameraPosPlayers5`))
    (:`6`
      (`self.SetArmLengthPlayers6`)
      (`self.SetCameraPosPlayers6`))))

(fn `ClassSetup`
  (bind _asbasket_ball_game_mode (cast `/Game/BasketBallGameMode` (`GameplayStatics.GetGameMode`)))
  (bind _output_get (set `self.BP_Gamemode` _asbasket_ball_game_mode))
  (set `self.PlayersReference` (`/Game/BasketBallGameMode.Players` _output_get))
  (bind _outactors (`GameplayStatics.GetAllActorsOfClass` "/Script/Engine.PlayerController"))
  (`PlayerController.SetViewTargetWithBlend` _outactors self 0.0 "VTBlend_Linear" 0.0 false)
  (for _array_element (`self.PlayersReference`)
    (switch `int` 0
      (:`0`
        (set `self.P1` _array_element))
      (:`1`
        (set `self.P2` _array_element))
      (:`2`
        (set `self.P3` _array_element))
      (:`3`
        (set `self.P4` _array_element))
      (:`4`
        (set `self.P5` _array_element))
      (:`5`
        (set `self.P6` _array_element)))))

(fn `SetArmLengthPlayers1`
  (bind _p1 (`self.P1`))
  (set `SpringArmComponent.TargetArmLength` (`KismetMathLibrary.FClamp` (`.MaxValue` (`KismetMathLibrary.MaxOfFloatArray` (`|MakeArray` (`self.GetDistanceTo` _p1 _p1)))) (`self.MinArmLength`) (`self.MaxArmLength`)) (`self.SpringArm`)))

(fn `SetArmLengthPlayers2`
  (set `SpringArmComponent.TargetArmLength` (`KismetMathLibrary.FClamp` (`.MaxValue` (`KismetMathLibrary.MaxOfFloatArray` (`|MakeArray` (`self.GetDistanceTo` (`self.P1`) (`self.P2`))))) (`self.MinArmLength`) (`self.MaxArmLength`)) (`self.SpringArm`)))

(fn `SetArmLengthPlayers3`
  (bind _p1 (`self.P1`))
  (bind _p2 (`self.P2`))
  (bind _p3 (`self.P3`))
  (set `SpringArmComponent.TargetArmLength` (`KismetMathLibrary.FClamp` (`.MaxValue` (`KismetMathLibrary.MaxOfFloatArray` (`|MakeArray` (`self.GetDistanceTo` _p1 _p2) (`self.GetDistanceTo` _p1 _p3) (`self.GetDistanceTo` _p2 _p3)))) (`self.MinArmLength`) (`self.MaxArmLength`)) (`self.SpringArm`)))

(fn `SetArmLengthPlayers4`
  (bind _p1 (`self.P1`))
  (bind _p2 (`self.P2`))
  (bind _p3 (`self.P3`))
  (bind _p4 (`self.P4`))
  (set `SpringArmComponent.TargetArmLength` (`KismetMathLibrary.FClamp` (`.MaxValue` (`KismetMathLibrary.MaxOfFloatArray` (`|MakeArray` (`self.GetDistanceTo` _p1 _p2) (`self.GetDistanceTo` _p1 _p3) (`self.GetDistanceTo` _p1 _p4) (`self.GetDistanceTo` _p2 _p3) (`self.GetDistanceTo` _p2 _p4) (`self.GetDistanceTo` _p3 _p4)))) (`self.MinArmLength`) (`self.MaxArmLength`)) (`self.SpringArm`)))

(fn `SetArmLengthPlayers5`
  (bind _p1 (`self.P1`))
  (bind _p2 (`self.P2`))
  (bind _p3 (`self.P3`))
  (bind _p4 (`self.P4`))
  (bind _p5 (`self.P5`))
  (set `SpringArmComponent.TargetArmLength` (`KismetMathLibrary.FClamp` (`.MaxValue` (`KismetMathLibrary.MaxOfFloatArray` (`|MakeArray` (`self.GetDistanceTo` _p1 _p2) (`self.GetDistanceTo` _p1 _p3) (`self.GetDistanceTo` _p1 _p4) (`self.GetDistanceTo` _p1 _p5) (`self.GetDistanceTo` _p2 _p3) (`self.GetDistanceTo` _p2 _p4) (`self.GetDistanceTo` _p2 _p5) (`self.GetDistanceTo` _p3 _p4) (`self.GetDistanceTo` _p3 _p5) (`self.GetDistanceTo` _p4 _p5)))) (`self.MinArmLength`) (`self.MaxArmLength`)) (`self.SpringArm`)))

(fn `SetArmLengthPlayers6`
  (bind _p1 (`self.P1`))
  (bind _p2 (`self.P2`))
  (bind _p3 (`self.P3`))
  (bind _p4 (`self.P4`))
  (bind _p5 (`self.P5`))
  (bind _p6 (`self.P6`))
  (set `SpringArmComponent.TargetArmLength` (`KismetMathLibrary.FClamp` (`.MaxValue` (`KismetMathLibrary.MaxOfFloatArray` (`|MakeArray` (`self.GetDistanceTo` _p1 _p2) (`self.GetDistanceTo` _p1 _p3) (`self.GetDistanceTo` _p1 _p4) (`self.GetDistanceTo` _p1 _p5) (`self.GetDistanceTo` _p1 _p6) (`self.GetDistanceTo` _p2 _p3) (`self.GetDistanceTo` _p2 _p4) (`self.GetDistanceTo` _p2 _p5) (`self.GetDistanceTo` _p2 _p6) (`self.GetDistanceTo` _p3 _p4) (`self.GetDistanceTo` _p3 _p5) (`self.GetDistanceTo` _p3 _p6) (`self.GetDistanceTo` _p4 _p5) (`self.GetDistanceTo` _p4 _p6) (`self.GetDistanceTo` _p5 _p6)))) (`self.MinArmLength`) (`self.MaxArmLength`)) (`self.SpringArm`)))

(fn `SetCameraPosPlayers1`
  (set `self.TargetPos` (+ (`self.K2_GetActorLocation` (`self.P1`)) (0.0 0.0 0.0)))
  (`self.K2_SetActorLocation` (`KismetMathLibrary.VInterpTo` (`self.PreviousPos`) (`self.TargetPos`) (`GameplayStatics.GetWorldDeltaSeconds`) (`self.InterpSpeed`)))
  (set `self.PreviousPos` (`self.K2_GetActorLocation`)))

(fn `SetCameraPosPlayers2`
  (set `self.TargetPos` (/ (+ (`self.K2_GetActorLocation` (`self.P1`)) (`self.K2_GetActorLocation` (`self.P2`))) (`KismetMathLibrary.Conv_IntToDouble` (`KismetArrayLibrary.Array_Length` (`self.PlayersReference`)))))
  (`self.K2_SetActorLocation` (`KismetMathLibrary.VInterpTo` (`self.PreviousPos`) (`self.TargetPos`) (`GameplayStatics.GetWorldDeltaSeconds`) (`self.InterpSpeed`)))
  (set `self.PreviousPos` (`self.K2_GetActorLocation`)))

(fn `SetCameraPosPlayers3`
  (set `self.TargetPos` (/ (+ (`self.K2_GetActorLocation` (`self.P1`)) (`self.K2_GetActorLocation` (`self.P2`)) (`self.K2_GetActorLocation` (`self.P3`))) (`KismetMathLibrary.Conv_IntToDouble` (`KismetArrayLibrary.Array_Length` (`self.PlayersReference`)))))
  (`self.K2_SetActorLocation` (`KismetMathLibrary.VInterpTo` (`self.PreviousPos`) (`self.TargetPos`) (`GameplayStatics.GetWorldDeltaSeconds`) (`self.InterpSpeed`)))
  (set `self.PreviousPos` (`self.K2_GetActorLocation`)))

(fn `SetCameraPosPlayers4`
  (set `self.TargetPos` (/ (+ (`self.K2_GetActorLocation` (`self.P1`)) (`self.K2_GetActorLocation` (`self.P2`)) (`self.K2_GetActorLocation` (`self.P3`)) (`self.K2_GetActorLocation` (`self.P4`))) (`KismetMathLibrary.Conv_IntToDouble` (`KismetArrayLibrary.Array_Length` (`self.PlayersReference`)))))
  (`self.K2_SetActorLocation` (`KismetMathLibrary.VInterpTo` (`self.PreviousPos`) (`self.TargetPos`) (`GameplayStatics.GetWorldDeltaSeconds`) (`self.InterpSpeed`)))
  (set `self.PreviousPos` (`self.K2_GetActorLocation`)))

(fn `SetCameraPosPlayers5`
  (set `self.TargetPos` (/ (+ (`self.K2_GetActorLocation` (`self.P1`)) (`self.K2_GetActorLocation` (`self.P2`)) (`self.K2_GetActorLocation` (`self.P3`)) (`self.K2_GetActorLocation` (`self.P4`)) (`self.K2_GetActorLocation` (`self.P5`))) (`KismetMathLibrary.Conv_IntToDouble` (`KismetArrayLibrary.Array_Length` (`self.PlayersReference`)))))
  (`self.K2_SetActorLocation` (`KismetMathLibrary.VInterpTo` (`self.PreviousPos`) (`self.TargetPos`) (`GameplayStatics.GetWorldDeltaSeconds`) (`self.InterpSpeed`)))
  (set `self.PreviousPos` (`self.K2_GetActorLocation`)))

(fn `SetCameraPosPlayers6`
  (set `self.TargetPos` (/ (+ (`self.K2_GetActorLocation` (`self.P1`)) (`self.K2_GetActorLocation` (`self.P2`)) (`self.K2_GetActorLocation` (`self.P3`)) (`self.K2_GetActorLocation` (`self.P4`)) (`self.K2_GetActorLocation` (`self.P5`)) (`self.K2_GetActorLocation` (`self.P6`))) (`KismetMathLibrary.Conv_IntToDouble` (`KismetArrayLibrary.Array_Length` (`self.PlayersReference`)))))
  (`self.K2_SetActorLocation` (`KismetMathLibrary.VInterpTo` (`self.PreviousPos`) (`self.TargetPos`) (`GameplayStatics.GetWorldDeltaSeconds`) (`self.InterpSpeed`)))
  (set `self.PreviousPos` (`self.K2_GetActorLocation`)))

(fn `UserConstructionScript`)